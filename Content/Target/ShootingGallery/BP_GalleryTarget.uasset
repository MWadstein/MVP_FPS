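; A shooting gallery target that shows its point value and either pops up, holds and retracts, or travels from spawn to end point.
; Rate-scaled timelines move the mesh, destroying the actor when the motion ends.
; Damage lowers health; at zero it sends its score to the game mode, increments the target manager's destroyed count and is destroyed.
; A dynamic material colors it by starting health, or by remaining health when enabled.
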(event `self.ReceiveBeginPlay`
  (`self.SetupTarget`)
  (switch `/Game/Target/ShootingGallery/Enum_Gallery_TargetType` (`self.TargetType`)
    (:`NewEnumerator0`
      (`self.HandlePopupTarget`))
    (:`NewEnumerator1`
      (`self.HandleMoveTarget`))))

(event `HandleMoveTarget`
  (`TimelineComponent.SetPlayRate` (`self.MoveTimeline`) (/ 1.0 (`self.Lifetime`)))
  (bind (_direction _lerp_0_1) (`Timeline|MoveTimeline` :!via `PlayFromStart`)
    (:`Update`
      (`SceneComponent.K2_SetWorldLocation` (`self.StaticMesh`) (`KismetMathLibrary.VLerp` (`self.SpawnPoint`) (`self.EndPoint`) _lerp_0_1) false false))
    (:`Finished`
      (`self.K2_DestroyActor`))))

(event `HandlePopupTarget`
  ;[1 1 1] What do we do when we are a popup target
  (`TimelineComponent.SetPlayRate` (`self.PopupTimeline`) (/ 1.0 (`self.PopupTime`)))
  (bind (_direction _lerp_0_1) (`Timeline|PopupTimeline` :!via `PlayFromStart`)
    (:`Update`
      (`SceneComponent.K2_SetWorldLocation` (`self.StaticMesh`) (`KismetMathLibrary.VLerp` (`self.SpawnPoint`) (`self.HoldPoint`) _lerp_0_1) false false))
    (:`Finished`
      (`KismetSystemLibrary.Delay` (`self.HoldTime`))
      (bind (_direction_2 _lerp_0_1_2) (`Timeline|PopdownTimeline` :!via `ReverseFromEnd`)
        (:`Update`
          (`SceneComponent.K2_SetWorldLocation` (`self.StaticMesh`) (`KismetMathLibrary.VLerp` (`self.SpawnPoint`) (`self.HoldPoint`) _lerp_0_1_2) false false))
        (:`Finished`
          (`self.K2_DestroyActor`))))))

(event `/Game/Interfaces/BPI_Damageable.HandleBeingDamaged`
  (params (WhoHitUs :type "Actor Object Reference") (DamageValue :type "Float (single-precision)"))
  (bind _output_get (set `self.HealthValue` (- (`self.HealthValue`) DamageValue)))
  (if (<= _output_get 0.0)
    (message `/Game/Interfaces/BPI_FPS-GameMode.HandleAddScore` (`GameplayStatics.GetGameMode`) (`self.Value`))
    (bind _outactors (`GameplayStatics.GetAllActorsOfClass` "/Game/Blueprints/ShootingGallery/BP_ShootingGallery_TargetManager.BP_ShootingGallery_TargetManager_C"))
    (`/Game/Blueprints/ShootingGallery/BP_ShootingGallery_TargetManager.IncrementTotalTargetsDestroyed` (`KismetArrayLibrary.Array_Get` _outactors))
    (`self.K2_DestroyActor`)
    (elif (`self.ChangeColorsWhenHit`)
      (`self.UpdateHealthColor`))))

(event `UpdateHealthColor`
  (bind _healthvalue (`self.HealthValue`))
  (bind _startinghealthvalue (`self.StartingHealthValue`))
  (`MaterialInstanceDynamic.SetVectorParameterValue` (`self.DynamicMatRef`) "HealthValueColor" (`KismetMathLibrary.LinearColorLerp` (struct :`R` 1.0 :`G` 0.01492 :`A` 1.0) (struct :`G` 1.0 :`A` 1.0) (/ (select `bool` (and (== _healthvalue _startinghealthvalue) (!= _startinghealthvalue 1.0)) :`false` (- _healthvalue 1.0) :`true` _healthvalue) (`self.StartingHealthValue`)))))

(fn `SetupTarget`
  (locals (LocalTargetColor :type "LinearColor Structure"))
  (`TextRenderComponent.K2_SetText` (`self.TextRender`) (`KismetTextLibrary.Conv_DoubleToText` (`self.Value`) "HalfToEven" false 1 324 0 0))
  (bind _returnvalue (`PrimitiveComponent.CreateDynamicMaterialInstance` (`self.StaticMesh`) 0 null))
  (set `self.DynamicMatRef` _returnvalue)
  (set `self.StartingHealthValue` (`self.HealthValue`))
  (if (`self.ChangeColorsWhenHit`)
    (`self.UpdateHealthColor`)
    (else
      (switch `int` (`KismetMathLibrary.FTrunc` (`self.HealthValue`))
        (:`Default`
          (set `local.LocalTargetColor` (struct :`R` 1.0 :`A` 1.0)))
        (:`1`
          (set `local.LocalTargetColor` (struct :`G` 1.0 :`A` 1.0)))
        (:`2`
          (set `local.LocalTargetColor` (struct :`R` 0.457433 :`G` 0.970142 :`B` 1.0 :`A` 1.0)))
        (:`3`
          (set `local.LocalTargetColor` (struct :`G` 0.235002 :`B` 1.0 :`A` 1.0)))
        (:`4`
          (set `local.LocalTargetColor` (struct :`R` 1.0 :`G` 0.536362 :`B` 0.18 :`A` 1.0))))
      (`MaterialInstanceDynamic.SetVectorParameterValue` (`self.DynamicMatRef`) "HealthValueColor" (`local.LocalTargetColor`)))))

(fn `UserConstructionScript`
  (`/Engine/EditorBlueprintResources/StandardMacros.IsValid` (`self.TestMesh`)
    (:`Is Valid`
      (`StaticMeshComponent.SetStaticMesh` (`self.StaticMesh`) (`self.TestMesh`)))))
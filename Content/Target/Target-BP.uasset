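; Target actor that players hit for score, shifting color from green to red as its health drops.
; BeginPlay creates a dynamic material for the cube and registers the target with the game mode.
; Each hit awards points to the hitter, subtracts damage and updates the color via a health-ratio lerp.
; At zero health it awards a bonus, notifies the game mode, plays a sound and destroys itself.
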(event `self.ReceiveBeginPlay`
  (set `self.StartingHealthValue` (`self.HealthValue`))
  (bind _returnvalue (`KismetMaterialLibrary.CreateDynamicMaterialInstance` "/Game/Materials/TargetMat.TargetMat"))
  (set `self.DynamicMat` _returnvalue)
  (`PrimitiveComponent.SetMaterial` (`self.Cube`) 0 (`self.DynamicMat`))
  (`self.SetColor`)
  (message `/Game/Interfaces/FPS-GameMode-BPI.AddTarget` (`GameplayStatics.GetGameMode`)))

(event `/Game/Target/Target-BP-BPI.HandleWasHit`
  (params (Hitter :type "Actor Object Reference") (DamageValue :type Integer))
  (set `self.Hitter` Hitter)
  (set `self.DamageValue` DamageValue)
  (message `/Game/Interfaces/FPS-Controller-BPI.HandleUpdateScore` (`self.Hitter`) (`self.TargetValue`))
  (set `self.HealthValue` (- (`self.HealthValue`) (`self.DamageValue`)))
  (`self.SetColor`)
  (if (<= (`self.HealthValue`) 0)
    (message `/Game/Interfaces/FPS-Controller-BPI.HandleUpdateScore` (`self.Hitter`) (`self.BonusValue`))
    (message `/Game/Interfaces/FPS-GameMode-BPI.RemoveTarget` (`GameplayStatics.GetGameMode`))
    (`GameplayStatics.PlaySoundAtLocation` null (`self.K2_GetActorLocation`))
    (`self.K2_DestroyActor`)))

(fn `SetColor`
  (`MaterialInstanceDynamic.SetVectorParameterValue` (`self.DynamicMat`) "Color" (`KismetMathLibrary.LinearColorLerp` (struct :`R` 1.0 :`A` 1.0) (struct :`G` 1.0 :`A` 1.0) (/ (`KismetMathLibrary.Conv_IntToDouble` (`self.HealthValue`)) (`KismetMathLibrary.Conv_IntToDouble` (`self.StartingHealthValue`)))))
  (return))

(fn `UserConstructionScript`)
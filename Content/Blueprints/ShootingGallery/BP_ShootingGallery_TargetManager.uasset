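; Shooting gallery manager that runs timed rounds of target waves and tracks spawned and destroyed target counts.
; Once BeginGame starts it, Tick compares elapsed time with each wave's time code in the nested TargetRounds data and spawns configured BP_GalleryTarget actors.
; After a round's last wave, function-name timers show upcoming-round or game-ending messages through the game mode, then reset for the next round or request game end.
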(event `BeginGame`
  ;[1 1 1] Begin Rounds Event
  (set `self.IsRunning` true))

(event `self.ReceiveTick`
  (params (DeltaSeconds :type "Float (single-precision)"))
  (bind _item_spawnarray (break `/Game/Blueprints/ShootingGallery/Struct_ShootingGallery_RoundInfo` (`KismetArrayLibrary.Array_Get` (`self.TargetRounds`) (`self.CurrentRoundNumber`))))
  (bind _item_spawnarray_2 (break `/Game/Blueprints/ShootingGallery/Struct_ShootingGallery_RoundInfo` (`KismetArrayLibrary.Array_Get` (`self.TargetRounds`) (`self.CurrentRoundNumber`))))
  (bind _item_spawnarray_3 (break `/Game/Blueprints/ShootingGallery/Struct_ShootingGallery_RoundInfo` (`KismetArrayLibrary.Array_Get` (`self.TargetRounds`) (`self.CurrentRoundNumber`))))
  (bind _item_timecode (break `/Game/Blueprints/ShootingGallery/Struct_ShootingGallery_SpawnInfo` (`KismetArrayLibrary.Array_Get` _item_spawnarray (`self.CurrentSpawnNumber`))))
  (bind (_item_timecode_2 _item_targetstospawn) (break `/Game/Blueprints/ShootingGallery/Struct_ShootingGallery_SpawnInfo` (`KismetArrayLibrary.Array_Get` _item_spawnarray_3 (`self.CurrentSpawnNumber`))))
  ;[1 1 1] Spawner for our Current Spawns for the Current Round
  (if (`self.IsRunning`)
    (bind _output_get (set `self.CurrentRunningTime` (+ DeltaSeconds (`self.CurrentRunningTime`))))
    (if (>= _output_get _item_timecode)
      (`self.UpdateRoundText`)
      (for _array_element _item_targetstospawn
        (bind _returnvalue (`|SpawnActorFromClass` "/Game/Target/ShootingGallery/BP_GalleryTarget.BP_GalleryTarget_C" (`KismetMathLibrary.MakeTransform` (`.SpawnPoint_19_9A36DBA644738A654AEB2480F9453161` (break `/Game/Blueprints/ShootingGallery/Struct_ShootingGallery_TargetInfo` _array_element)) (struct :`Yaw` 180.0)) "Undefined" "OverrideRootScale" null (break `/Game/Blueprints/ShootingGallery/Struct_ShootingGallery_TargetInfo` _array_element) (`.LifeTime_17_2E55AA434532AEE0AAE2098962394C34` (break `/Game/Blueprints/ShootingGallery/Struct_ShootingGallery_TargetInfo` _array_element)) (`.Value_18_2B21BD0F40BEBFB76D35CEA00B8FEE8E` (break `/Game/Blueprints/ShootingGallery/Struct_ShootingGallery_TargetInfo` _array_element)) (`.SpawnPoint_19_9A36DBA644738A654AEB2480F9453161` (break `/Game/Blueprints/ShootingGallery/Struct_ShootingGallery_TargetInfo` _array_element)) (`.HoldPoint_20_8EE45A1C4B2F6341B57FF6B0B62BDD5C` (break `/Game/Blueprints/ShootingGallery/Struct_ShootingGallery_TargetInfo` _array_element)) (`.EndPoint_21_1F8C42854135799956D116A9E0AEB1B6` (break `/Game/Blueprints/ShootingGallery/Struct_ShootingGallery_TargetInfo` _array_element)) (`.HoldTime_26_342EFC194220F4A9315BD39EAF2D1F82` (break `/Game/Blueprints/ShootingGallery/Struct_ShootingGallery_TargetInfo` _array_element)) (`.PopupTime_27_C24184984E7CD45574BC55BACEF44812` (break `/Game/Blueprints/ShootingGallery/Struct_ShootingGallery_TargetInfo` _array_element)) (`.HealthValue_31_0A1A5EC540E11B90CC35B8AA22795606` (break `/Game/Blueprints/ShootingGallery/Struct_ShootingGallery_TargetInfo` _array_element))))
        (`StaticMeshComponent.SetStaticMesh` (`/Game/Target/ShootingGallery/BP_GalleryTarget.StaticMesh` _returnvalue) (`.TargetMesh_16_13F4031E45E6F599C35816A91A9D4DA9` (break `/Game/Blueprints/ShootingGallery/Struct_ShootingGallery_TargetInfo` _array_element)))
        (`/Engine/EditorBlueprintResources/StandardMacros.IncrementInt` (`self.TotalTargetSpawned`)))
      (`/Engine/EditorBlueprintResources/StandardMacros.IncrementInt` (`self.CurrentSpawnNumber`)
        (:`  `
          (if (< (`KismetArrayLibrary.Array_LastIndex` _item_spawnarray_2) (`self.CurrentSpawnNumber`))
            (`/Engine/EditorBlueprintResources/StandardMacros.IncrementInt` (`self.CurrentRoundNumber`)
              (:`  `
                (if (< (`KismetArrayLibrary.Array_LastIndex` (`self.TargetRounds`)) (`self.CurrentRoundNumber`))
                  (set `self.IsRunning` false)
                  (`KismetSystemLibrary.K2_SetTimer` null "ShowGameOverSoonMessage" (/ (`self.DelayBetweenRounds`) 2.0))
                  (else
                    (set `self.IsRunning` false)
                    (`KismetSystemLibrary.K2_SetTimer` null "HandleDelayBetweenRounds" (`self.DelayBetweenRounds`))
                    (`KismetSystemLibrary.K2_SetTimer` null "ShowNextRoundStartingSoonMessage" (/ (`self.DelayBetweenRounds`) 2.0))))))
            (else
              (`KismetSystemLibrary.PrintString` "Spawns done, more to go"))))))))

(event `HandleDelayBetweenRounds`
  ;[1 1 1] Handle the delay and resetting of our variables between rounds
  (set `self.CurrentRunningTime` 0.0)
  (set `self.CurrentSpawnNumber` 0)
  (set `self.IsRunning` true))

(event `ShowNextRoundStartingSoonMessage`
  (message `/Game/Interfaces/BPI_ShootingGallery_GameMode.UpdateRoundText` (`GameplayStatics.GetGameMode`) (`|FormatText` "Round {num} Starting Soon" (+ (`self.CurrentRoundNumber`) 1))))

(event `ShowGameOverSoonMessage`
  (message `/Game/Interfaces/BPI_ShootingGallery_GameMode.UpdateRoundText` (`GameplayStatics.GetGameMode`) "Game Ending Soon")
  (`KismetSystemLibrary.Delay` (/ (`self.DelayBetweenRounds`) 2.0))
  (message `/Game/Interfaces/BPI_FPS-GameMode.GameWantsToEnd` (`GameplayStatics.GetGameMode`)))

(event `IncrementTotalTargetsDestroyed`
  (`/Engine/EditorBlueprintResources/StandardMacros.IncrementInt` (`self.TotalTargetsDestroyed`)))

(fn `UserConstructionScript`)
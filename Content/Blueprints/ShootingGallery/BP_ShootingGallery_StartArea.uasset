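; Start trigger area for the shooting gallery that lets the player begin the game by pressing E inside it.
; Box overlap events set an in-area flag and show or clear a "Press E" HUD prompt, without filtering which actor overlaps.
; The E key checks that flag, then messages the game mode to start and clears the prompt, with all communication going through game mode message calls.
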(event `Key|E`
  (params (Key :type "Key Structure" :default "AnyKey"))
  (:`Pressed`
    (if (`self.IsInStartArea`)
      (message `/Game/Interfaces/BPI_FPS-GameMode.PlayerWantsToStart` (`GameplayStatics.GetGameMode`))
      (message `/Game/Interfaces/BPI_FPS-GameMode.UpdatePopupTextOnHUD` (`GameplayStatics.GetGameMode`) ""))))

(event `self.Box.OnComponentBeginOverlap`
  (params (OverlappedComponent :type "PrimitiveComponent Object Reference") (OtherActor :type "Actor Object Reference") (OtherComp :type "PrimitiveComponent Object Reference") (OtherBodyIndex :type Integer) (bFromSweep :type Boolean) (SweepResult :type "HitResult Structure (by ref)"))
  (set `self.IsInStartArea` true)
  (message `/Game/Interfaces/BPI_FPS-GameMode.UpdatePopupTextOnHUD` (`GameplayStatics.GetGameMode`) "Press \"E\" To Start"))

(event `self.Box.OnComponentEndOverlap`
  (params (OverlappedComponent :type "PrimitiveComponent Object Reference") (OtherActor :type "Actor Object Reference") (OtherComp :type "PrimitiveComponent Object Reference") (OtherBodyIndex :type Integer))
  (set `self.IsInStartArea` false)
  (message `/Game/Interfaces/BPI_FPS-GameMode.UpdatePopupTextOnHUD` (`GameplayStatics.GetGameMode`) ""))

(fn `UserConstructionScript`)
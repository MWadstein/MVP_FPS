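; BP_Weapon_Projectile is a weapon projectile that damages actors it collides with.
; On a collision hit, it sends its truncated damage value to actors implementing BPI_Damageable, then destroys itself.
; Hits on other actors destroy it only when its ProjectileMovement is not set to bounce.
; A setter event updates the damage value, and the CollisionIsOverriden flag disables this default hit handling.
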(event `self.Collision.OnComponentHit`
  (params (HitComponent :type "PrimitiveComponent Object Reference") (OtherActor :type "Actor Object Reference") (OtherComp :type "PrimitiveComponent Object Reference") (NormalImpulse :type "Vector Structure") (Hit :type "HitResult Structure (by ref)"))
  (if (`self.CollisionIsOverriden`)
    _
    (elif (`KismetSystemLibrary.DoesImplementInterface` OtherActor "/Game/Interfaces/BPI_Damageable.BPI_Damageable_C")
      (message `/Game/Target/Target-BP-BPI.HandleWasHit` OtherActor self (`KismetMathLibrary.FTrunc` (`self.DamageValue`)))
      (`self.K2_DestroyActor`)
      (elif (not (`ProjectileMovementComponent.bShouldBounce` (`self.ProjectileMovement`)))
        (`self.K2_DestroyActor`)))))

(event `/Game/Interfaces/BPI_Weapon_Projectile.SetDamageValue`
  (params (NewValue :type "Float (single-precision)"))
  (set `self.DamageValue` NewValue))

(fn `UserConstructionScript`)
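; Weapon pickup actor that gives its named weapon to any overlapping actor implementing the FPSCharacterBPI interface.
; The construction script looks up WeaponName in the weapon data table, then sets the ground mesh from that row and sizes the trigger box from CollisionExtents.
; On box overlap it sends the weapon name through the interface's AddWeaponToPlayer message and destroys itself.
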(event `self.Box.OnComponentBeginOverlap`
  (params (OverlappedComponent :type "PrimitiveComponent Object Reference") (OtherActor :type "Actor Object Reference") (OtherComp :type "PrimitiveComponent Object Reference") (OtherBodyIndex :type Integer) (bFromSweep :type Boolean) (SweepResult :type "HitResult Structure (by ref)"))
  (if (`KismetSystemLibrary.DoesImplementInterface` OtherActor "/Game/Interfaces/FPS-Character-BPI.FPS-Character-BPI_C")
    (message `/Game/Interfaces/FPS-Character-BPI.AddWeaponToPlayer` OtherActor (`self.WeaponName`))
    (`self.K2_DestroyActor`)))

(fn `UserConstructionScript`
  (bind _returnvalue (`|GetDataTableRow` "/Game/Data/Weapon_Data_Table.Weapon_Data_Table" (`self.WeaponName`))
    (:`then`
      (`StaticMeshComponent.SetStaticMesh` (`self.StaticMesh`) (`.GroundMesh_15_CB5129374EE9DA0167625AB8EDE34648` (break `/Game/Data/Weapon_Data_Struct` _returnvalue)))
      (`BoxComponent.SetBoxExtent` (`self.Box`) (`self.CollisionExtents`) true))))